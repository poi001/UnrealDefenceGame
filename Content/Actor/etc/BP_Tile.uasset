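; BP_Tile is a clickable tile actor that highlights on mouse hover and responds to selection clicks.
; Cursor events on its Tile component switch between the select and basic materials, and a click calls OnClickedTile.
; All three responses run only while IsSelecting is false.
; The material and click functions are called here but not defined in this graph, and the construction script is empty.
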(event `self.Tile.OnBeginCursorOver`
  (params (TouchedComponent :type "PrimitiveComponent Object Reference"))
  (if (not (`self.IsSelecting`))
    (`self.SetMaterialSelect`)))

(event `self.Tile.OnEndCursorOver`
  (params (TouchedComponent :type "PrimitiveComponent Object Reference"))
  (if (not (`self.IsSelecting`))
    (`self.SetMaterialBasic`)))

(event `self.Tile.OnClicked`
  (params (TouchedComponent :type "PrimitiveComponent Object Reference") (ButtonPressed :type "Key Structure"))
  (if (not (`self.IsSelecting`))
    (`self.OnClickedTile`)))

(fn `UserConstructionScript`)