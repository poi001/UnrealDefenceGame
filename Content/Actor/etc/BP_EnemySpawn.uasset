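; BP_EnemySpawn is a spawner actor that repeatedly spawns zombies at its own transform on a timer.
; Tick accumulates elapsed time until it reaches FSpawnTime, then spawns BP_BossZombie when DGGameStateBase's CurrentLevel is 10, otherwise BP_Zombie.
; After each spawn, the timer restarts from an offset that grows with CurrentLevel, shortening the wait at higher levels.
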(event `self.ReceiveBeginPlay`)

(event `self.ReceiveTick`
  (params (DeltaSeconds :type "Float (single-precision)"))
  (bind _returnvalue (`self.GetTransform` self))
  (set `self.Delta Seconds` (+ DeltaSeconds (`self.Delta Seconds`)))
  (if (>= (`self.Delta Seconds`) (`self.fSpawnTime`))
    (`|ExecutionSequence`
      (:`then_0`
        (bind _asdggame_state_base (cast `DGGameStateBase` (`GameplayStatics.GetGameState`)))
        (if (== (`DGGameStateBase.CurrentLevel` _asdggame_state_base) 10)
          (`|SpawnActorFromClass` "/Game/Actor/Enemy/Blueprint/BossZombie/BP_BossZombie.BP_BossZombie_C" _returnvalue "AdjustIfPossibleButAlwaysSpawn" "MultiplyWithRoot" null null)
          (else
            (`|SpawnActorFromClass` "/Game/Actor/Enemy/Blueprint/Zombie/BP_Zombie.BP_Zombie_C" _returnvalue "AdjustIfPossibleButAlwaysSpawn" "MultiplyWithRoot" null null))))
      (:`then_1`
        (bind _asdggame_state_base_2 (cast `DGGameStateBase` (`GameplayStatics.GetGameState`)))
        (set `self.Delta Seconds` (- (* (`KismetMathLibrary.Conv_IntToDouble` (`DGGameStateBase.CurrentLevel` _asdggame_state_base_2)) 0.1) 0.1))))))

(fn `UserConstructionScript`)